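; BP_Zombie_Auto4 is a zombie enemy that chases the player and deals fixed damage when it overlaps them.
; Tick reissues AIMoveTo toward the player character every frame, and ActorBeginOverlap calls OnDamaged on the player.
; ZombieApplyDamage subtracts from HP, while BeginPlay initializes a separately named CurHp from MaxHp.
; OnDie, which nothing here calls, enables mesh physics for a ragdoll-style collapse and destroys the capsule collision.
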(event Custom|Destroy%20Collision
  ;[1 1 1] 좀비가 죽고난 후의 충돌 제거
  (Components|DestroyComponent (Variables|Default|GetCapsuleComponent)))

(event EventBeginPlay
  ;[1 1 1] Zombie가 생성될 때 MaxHP 값을 Set
  (Variables|Default|SetCurHp (Variables|Default|GetMaxHp)))

(event Collision|EventActorBeginOverlap
  (params (OtherActor :type Actor%20Object%20Reference))
  ;[1 1 1] Zombie 가 Player 에게 닿았을 때 On Damaged
  (bind _asbp_plyaer_character (Utilities|Casting|CastToBP_PlyaerCharacter))
  (Class|PlayerCharacter|OnDamaged _asbp_plyaer_character 5))

(event EventTick
  (params (DeltaSeconds :type Float%20%28single-precision%29))
  ;[1 1 1] 매 프레임마다 한 번씩 실행
  (AI|AIMoveTo self "0, 0, 0" (Game|GetPlayerCharacter 0) 5.0 false))

(event EventOnDie
  ;[1 1 1] 좀비가 죽었을 때 발생하는 이펙트(쓰러짐, 터짐 등)
  (Physics|SetSimulatePhysics (Variables|Character|GetMesh) true)
  (CallFunction|DestroyCollision))

(fn ConstructionScript)

(fn ZombieApplyDamage
  (params (Damage :type Integer))
  (Variables|Default|SetHP (- (Variables|Default|GetHP) Damage))
  (return (Variables|Default|GetHP)))
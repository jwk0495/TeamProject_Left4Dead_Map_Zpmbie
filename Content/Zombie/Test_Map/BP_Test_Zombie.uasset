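; BP_Test_Zombie is a test zombie enemy that chases the player and damages them on contact.
; PawnSensing sets PawnSee on sighting a pawn and triggers AIMoveTo toward player character 0.
; Capsule overlap with BP_PlyaerCharacter calls its OnDamaged with a fixed amount.
; BeginPlay initialises health to MaxHp; OnDie ragdolls the mesh and destroys the capsule, though nothing in this Blueprint calls it or reduces health.
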(event OnSeePawn(PawnSensing)
  (params (Pawn :type Pawn%20Object%20Reference))
  (Variables|Default|SetpawnSee true)
  (CallFunction|FollowPlayer))

(event OnComponentBeginOverlap(CapsuleComponent)
  (params (OverlappedComponent :type Primitive%20Component%20Object%20Reference) (OtherActor :type Actor%20Object%20Reference) (OtherComp :type Primitive%20Component%20Object%20Reference) (OtherBodyIndex :type Integer) (bFromSweep :type Boolean) (SweepResult :type Hit%20Result%20Structure%20%28by%20ref%29))
  (bind _asbp_plyaer_character (Utilities|Casting|CastToBP_PlyaerCharacter OtherActor))
  (Class|PlayerCharacter|OnDamaged _asbp_plyaer_character 5))

(event Custom|Follow%20Player
  (if (Variables|Default|GetpawnSee)
    (AI|AIMoveTo self "0, 0, 0" (Game|GetPlayerCharacter 0) 5.0 false)))

(event Custom|Destory%20Collision
  ;[1 1 1] Zombie가 죽고난 후 Collision 제거
  (Components|DestroyComponent (Variables|Default|GetCapsuleComponent)))

(event EventBeginPlay
  ;[1 1 1] Zombie가 생성될 때 Max Hp값을 Setting
  (Variables|Default|SetCurHp (Variables|Default|GetMaxHp)))

(event Collision|EventActorBeginOverlap
  (params (OtherActor :type Actor%20Object%20Reference)))

(event EventTick
  (params (DeltaSeconds :type Float%20%28single-precision%29)))

(event EventOnDie
  ;[1 1 1] Zombie가 죽었을 때 나타나는 이펙트
  (Physics|SetSimulatePhysics (Variables|Character|GetMesh) true)
  (CallFunction|DestoryCollision))

(fn ConstructionScript)
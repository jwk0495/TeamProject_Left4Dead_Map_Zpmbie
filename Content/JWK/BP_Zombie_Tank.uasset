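; BP_Zombie_Tank is the tank zombie enemy, which chases the player and attacks in melee.
; On spawn it fills HP and, if PawnSensing's SeePawns setting is on, starts following the player; actually seeing a pawn raises its walk speed.
; AIMoveTo and a swipe montage loop into each other, with montage notifies triggering a sphere overlap that damages the player.
; Death ragdolls the mesh, destroys the capsule and increments the GameMode kill count.
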(event OnSeePawn(PawnSensing)
  (params (Pawn :type Pawn%20Object%20Reference))
  ;[1 1 1] Zombie가 Player를 발견 시 이동속도 Set
  (Variables|/Script/Engine.CharacterMovementComponent|SetMaxWalkSpeed (Variables|Character|GetCharacterMovement) 8e+02))

(event Custom|Destroy%20Collision%20Tank
  ;[1 1 1] Zombie가 죽고난 후 Collision 제거
  (Components|DestroyComponent (Variables|Default|GetCapsuleComponent)))

(event Custom|Follow%20Player%20Tank
  ;[1 1 1] TankZombie가 Player를 발견할 시 Player를 따라감
  (AI|AIMoveTo self "0, 0, 0" (Game|GetPlayerCharacter 0) 2e+01 false
    (:OnSuccess
      (CallFunction|AttackPlayerTank))
    (:OnFail
      (CallFunction|FollowPlayerTank))))

(event Custom|Attack%20Player%20Tank
  ;[1 1 1] TankZombie가 Player를 공격하는 애니메이션(Montage) 적용
  (Animation|Montage|PlayMontage (Variables|Character|GetMesh) "/Game/JWK/Zombie_Model/Zombie_Animation/Zombie_Tank_Anim/Montage_Tank_Attack_Swiping.Montage_Tank_Attack_Swiping"
    (:OnCompleted
      (CallFunction|FollowPlayerTank))
    (:OnNotifyBegin
      (bind (_outactors _returnvalue) (Collision|SphereOverlapActors (Transformation|GetWorldLocation (Variables|Default|GetArrow1)) 1.2e+02 (Utilities|Array|MakeArray "ObjectTypeQuery3") "/Game/PKH/BP/BP_PlyaerCharacter.BP_PlyaerCharacter_C" (Utilities|Array|MakeArray self)))
      (if _returnvalue
        (for _array_element _outactors
          (bind _asbp_plyaer_character (Utilities|Casting|CastToBP_PlyaerCharacter _array_element))
          (Class|PlayerCharacter|OnDamaged _asbp_plyaer_character 30))))))

(event EventBeginPlay
  ;[1 1 1] Zombie가 생성될 때 Max Hp값을 Set
  (Variables|Default|SetCurHp (Variables|Default|GetMaxHp))
  (if (Variables|/Script/AIModule.PawnSensingComponent|GetbSeePawns (Variables|Default|GetPawnSensing))
    (CallFunction|FollowPlayerTank)))

(event Collision|EventActorBeginOverlap
  (params (OtherActor :type Actor%20Object%20Reference)))

(event EventTick
  (params (DeltaSeconds :type Float%20%28single-precision%29)))

(event EventOnDie
  ;[1 1 1] Zombie가 죽고난 후 Collision 제거
  (Physics|SetSimulatePhysics (Variables|Character|GetMesh) true)
  (CallFunction|DestroyCollisionTank)
  (bind _asmy_game_mode (Utilities|Casting|CastToMyGameMode (Game|GetGameMode)))
  (Class|MyGameMode|KillCountPlus _asmy_game_mode))

(fn ConstructionScript)
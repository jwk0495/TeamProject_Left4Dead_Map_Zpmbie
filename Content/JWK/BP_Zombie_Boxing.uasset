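; Boxing zombie enemy that chases the player and punches in melee, with sight from PawnSensing raising its walk speed.
; BeginPlay initializes health and, if SeePawns is enabled, starts an AIMoveTo chase that retries on failure and attacks on arrival.
; The attack montage's notify applies damage through a sphere overlap at an arrow component, then resumes chasing on completion.
; Death enables ragdoll physics, removes the capsule and increments the game mode's kill count.
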(event OnSeePawn(PawnSensing)
  (params (Pawn :type Pawn%20Object%20Reference))
  ;[1 1 1] Zombie가 Player를 발견 시 이동속도 Set
  (Variables|/Script/Engine.CharacterMovementComponent|SetMaxWalkSpeed (Variables|Character|GetCharacterMovement) 4.5e+02))

(event Custom|Destroy%20Collision
  ;[1 1 1] BoxingZombie가 죽고난 후 Collision 제거
  (Components|DestroyComponent (Variables|Default|GetCapsuleComponent)))

(event Custom|Follow%20Player%20Boxing
  ;[1 1 1] BoxingZombie가 Player를 발견할 시 Player를 따라감
  (AI|AIMoveTo self "0, 0, 0" (Game|GetPlayerCharacter 0) 5.0 false
    (:OnSuccess
      (CallFunction|AttackPlayerCrawl))
    (:OnFail
      (CallFunction|FollowPlayerBoxing))))

(event Custom|AttackPlayer%20Crawl
  ;[1 1 1] BoxingZombie가 Player를 공격하는 애니메이션(Montage) 적용
  (Animation|Montage|PlayMontage (Variables|Character|GetMesh) "/Game/JWK/Zombie_Model/Zombie_Animation/Zombie_Boxing_Anim/Montage_Boxing_Zombie.Montage_Boxing_Zombie"
    (:OnCompleted
      (CallFunction|FollowPlayerBoxing))
    (:OnNotifyBegin
      (bind _outactors (Collision|SphereOverlapActors (Transformation|GetWorldLocation (Variables|Default|GetArrow1)) 8e+01 (Utilities|Array|MakeArray "ObjectTypeQuery3") "/Game/PKH/BP/BP_PlyaerCharacter.BP_PlyaerCharacter_C" (Utilities|Array|MakeArray self)))
      (if true
        (for _array_element _outactors
          (bind _asbp_plyaer_character (Utilities|Casting|CastToBP_PlyaerCharacter _array_element))
          (Class|PlayerCharacter|OnDamaged _asbp_plyaer_character 20))))))

(event EventOnDie
  ;[1 1 1] BoxingZombie가 죽고난 후 Collision 제거
  (Physics|SetSimulatePhysics (Variables|Character|GetMesh) true)
  (CallFunction|DestroyCollision)
  (bind _asmy_game_mode (Utilities|Casting|CastToMyGameMode (Game|GetGameMode)))
  (Class|MyGameMode|KillCountPlus _asmy_game_mode))

(event EventBeginPlay
  ;[1 1 1] BoxinglZombie가 생성될 때 MaxHP 값을 Set,  Zombie의 시야각 안에 들어올 때 Player 추격
  (Variables|Default|SetCurHp (Variables|Default|GetMaxHp))
  (if (Variables|/Script/AIModule.PawnSensingComponent|GetbSeePawns (Variables|Default|GetPawnSensing))
    (CallFunction|FollowPlayerBoxing)))

(fn ConstructionScript)
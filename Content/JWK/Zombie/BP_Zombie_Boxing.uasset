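; Boxing zombie enemy that chases the player and throws melee attacks.
; If pawn sensing is enabled at BeginPlay, it loops AIMoveTo into an attack montage, while seeing a pawn raises its walk speed.
; Montage notifies run a sphere overlap at an arrow component to damage the player.
; On death it ragdolls, destroys its capsule, plays a sound and increments the game mode's kill count.
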(event OnSeePawn(PawnSensing_Boxing)
  (params (Pawn :type Pawn%20Object%20Reference))
  ;[1 1 1] Zombie가 Player를 발견 시 이동속도 Set
  (Variables|/Script/Engine.CharacterMovementComponent|SetMaxWalkSpeed (Variables|Character|GetCharacterMovement) 4.5e+02))

(event Custom|Destroy%20Collision%20Boxing
  (bind _capsulecomponent (Variables|Default|GetCapsuleComponent))
  ;[1 1 1] BoxingZombie가 죽고난 후 Collision 제거
  (Utilities|IsValid _capsulecomponent
    (:Is%20Valid
      (Components|DestroyComponent _capsulecomponent))))

(event Custom|Follow%20Player%20Boxing
  ;[1 1 1] BoxingZombie가 Player를 발견할 시 Player를 따라감
  (AI|AIMoveTo self "0, 0, 0" (Game|GetPlayerCharacter 0) 2e+01 false
    (:OnSuccess
      (CallFunction|AttackPlayerBoxing)
      (bind _asbp_plyaer_character (Utilities|Casting|CastToBP_PlyaerCharacter (Game|GetPlayerCharacter 0)))
      (bind _returnvalue (Class|PlayerCharacter|IsDeadorClear _asbp_plyaer_character))
      (if (not _returnvalue)
        (Audio|PlaySound2D "/Game/JWK/Zombie/Sound/Boxing/Boxing_Attack/Boxing_Random_Attack.Boxing_Random_Attack" 1.0 1.0 0.0 0 0)))
    (:OnFail
      (CallFunction|FollowPlayerBoxing))))

(event Custom|AttackPlayer%20Boxing
  ;[1 1 1] BoxingZombie가 Player를 공격하는 애니메이션(Montage) 적용
  (Animation|Montage|PlayMontage (Variables|Character|GetMesh) "/Game/JWK/Zombie/Zombie_Model/Zombie_Animation/Zombie_Boxing_Anim/Montage_Boxing_Zombie.Montage_Boxing_Zombie"
    (:OnCompleted
      (CallFunction|FollowPlayerBoxing))
    (:OnNotifyBegin
      (bind (_outactors _returnvalue) (Collision|SphereOverlapActors (Transformation|GetWorldLocation (Variables|Default|GetArrow1)) 8e+01 (Utilities|Array|MakeArray "ObjectTypeQuery3") "/Game/PKH/BP/BP_PlyaerCharacter.BP_PlyaerCharacter_C" (Utilities|Array|MakeArray self)))
      (if _returnvalue
        (for _array_element _outactors
          (bind _asbp_plyaer_character (Utilities|Casting|CastToBP_PlyaerCharacter _array_element))
          (Class|PlayerCharacter|OnDamaged _asbp_plyaer_character 20))))))

(event EventOnDie
  ;[1 1 1] BoxingZombie가 죽고난 후 Collision 제거
  (Physics|SetSimulatePhysics (Variables|Character|GetMesh) true)
  (CallFunction|DestroyCollisionBoxing)
  (Audio|PlaySound2D "/Game/JWK/Zombie/Sound/Boxing/Boxing_Death.Boxing_Death" 0.7 0.7 0.7 0 0)
  (bind _asmy_game_mode (Utilities|Casting|CastToMyGameMode (Game|GetGameMode)))
  (Class|MyGameMode|KillCountPlus _asmy_game_mode))

(event EventBeginPlay
  ;[1 1 1] BoxinglZombie가 생성될 때 MaxHP 값을 Set,  Zombie의 시야각 안에 들어올 때 Player 추격
  (Variables|Default|SetCurHp (Variables|Default|GetMaxHp))
  (if (Variables|/Script/AIModule.PawnSensingComponent|GetbSeePawns (Variables|Default|GetPawnSensing_Boxing))
    (CallFunction|FollowPlayerBoxing)))

(fn ConstructionScript)
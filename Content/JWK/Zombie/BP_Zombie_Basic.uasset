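; BP_Zombie_Basic is the basic zombie enemy that chases and melees the player character.
; It starts an AI MoveTo chase at spawn if pawn sensing has sight enabled, retries on failure, and speeds up on seeing a pawn.
; On arrival it plays an attack montage whose notify triggers a sphere-overlap damage check, then resumes chasing.
; On death it ragdolls, destroys its capsule, plays a sound and increments the GameMode kill count.
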(event OnSeePawn(PawnSensing)
  (params (Pawn :type Pawn%20Object%20Reference))
  ;[0.03277 1 0] Zombie가 Player를 발견 시 이동속도 Set
  (Variables|/Script/Engine.CharacterMovementComponent|SetMaxWalkSpeed (Variables|Character|GetCharacterMovement) 3e+02))

(event Custom|Destroy%20Collision%20Basic
  (bind _capsulecomponent (Variables|Default|GetCapsuleComponent))
  ;[1 0 0] Zombie가 죽고난 후 Collision 제거
  (Utilities|IsValid _capsulecomponent
    (:Is%20Valid
      (Components|DestroyComponent _capsulecomponent))))

(event Custom|Follow%20Player%20Basic
  ;[0 0.8138 1] BasicZombie가 Player를 발견할 시 Player를 따라감
  (AI|AIMoveTo self "0, 0, 0" (Game|GetPlayerCharacter 0) 2e+01 false
    (:OnSuccess
      (CallFunction|AttackPlayerBasic)
      ;;[1 1 1] Player가 죽거나 클리어 했을 때 Zombie의 공격 사운드 제거
      (bind _asbp_plyaer_character (Utilities|Casting|CastToBP_PlyaerCharacter (Game|GetPlayerCharacter 0)))
      (bind _returnvalue (Class|PlayerCharacter|IsDeadorClear _asbp_plyaer_character))
      (if (not _returnvalue)
        (Audio|PlaySound2D "/Game/JWK/Zombie/Sound/Basic/Basic_Attack/Basic_Random_Attack.Basic_Random_Attack" 0.5 0.5 0.0 0 0)))
    (:OnFail
      (CallFunction|FollowPlayerBasic))))

(event Custom|AttackPlayer%20Basic
  ;[1 0 0] BasicZombie가 Player를 공격하는 애니메이션(Montage) 적용
  (Animation|Montage|PlayMontage (Variables|Character|GetMesh) "/Game/JWK/Zombie/Zombie_Model/Zombie_Animation/Zombie_Basic_Anims/Montage_Basic_Zombie_Attack.Montage_Basic_Zombie_Attack"
    (:OnCompleted
      (CallFunction|FollowPlayerBasic))
    (:OnNotifyBegin
      (bind (_outactors _returnvalue) (Collision|SphereOverlapActors (Transformation|GetWorldLocation (Variables|Default|GetArrow1)) 8e+01 (Utilities|Array|MakeArray "ObjectTypeQuery3") "/Game/PKH/BP/BP_PlyaerCharacter.BP_PlyaerCharacter_C" (Utilities|Array|MakeArray self)))
      (if _returnvalue
        (for _array_element _outactors
          (bind _asbp_plyaer_character (Utilities|Casting|CastToBP_PlyaerCharacter _array_element))
          (Class|PlayerCharacter|OnDamaged _asbp_plyaer_character 10))))))

(event EventBeginPlay
  ;[0.04246 1 0.05443] Zombie가 생성될 때 Max HP 값을 Set,     Zombie의 시야각 안에 들어올 때 Player 추격
  (Variables|Default|SetCurHp (Variables|Default|GetMaxHp))
  (if (Variables|/Script/AIModule.PawnSensingComponent|GetbSeePawns (Variables|Default|GetPawnSensing))
    (CallFunction|FollowPlayerBasic)))

(event EventOnDie
  ;[1 0 0] Zombie가 죽고난 후 Collision 제거
  (Physics|SetSimulatePhysics (Variables|Character|GetMesh) true)
  (CallFunction|DestroyCollisionBasic)
  (Audio|PlaySound2D "/Game/JWK/Zombie/Sound/Basic/Basic_Death/Basic_Random_Death.Basic_Random_Death" 0.2 0.2 0.0 0 0)
  (bind _asmy_game_mode (Utilities|Casting|CastToMyGameMode (Game|GetGameMode)))
  (Class|MyGameMode|KillCountPlus _asmy_game_mode))

(fn ConstructionScript)
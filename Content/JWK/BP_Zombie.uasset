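; BP_Zombie is an enemy character that chases the player and deals damage on contact.
; PawnSensing sets a seen flag, raises walk speed and starts AIMoveTo toward the player character.
; Capsule hits call OnDamaged on the player; the trailing 3-second Delay does not gate repeat damage.
; HP starts at max, and OnDie ragdolls the mesh and destroys the capsule, though nothing here calls it.
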(event OnSeePawn(PawnSensing)
  (params (Pawn :type Pawn%20Object%20Reference))
  ;[1 1 1] Player를 발견했을 때 Player를 따라감
  (Variables|Default|SetpawnSee true)
  (CallFunction|FollowPlayer))

(event OnComponentHit(CapsuleComponent)
  (params (HitComponent :type Primitive%20Component%20Object%20Reference) (OtherActor :type Actor%20Object%20Reference) (OtherComp :type Primitive%20Component%20Object%20Reference) (NormalImpulse :type Vector :default "0, 0, 0") (Hit :type Hit%20Result%20Structure%20%28by%20ref%29))
  ;[1 1 1] Zombie와 Collision이 발생하면 3초 간격으로 Player가 대미지를 입음
  (bind _asbp_plyaer_character (Utilities|Casting|CastToBP_PlyaerCharacter OtherActor))
  (Class|PlayerCharacter|OnDamaged _asbp_plyaer_character 5)
  (Utilities|FlowControl|Delay 3.0))

(event Custom|Destroy%20Collision
  ;[1 1 1] Zombie가 죽고난 후 Collision 제거
  (Components|DestroyComponent (Variables|Default|GetCapsuleComponent)))

(event Custom|FollowPlayer
  ;[1 1 1] Player를 따라감
  (Variables|/Script/Engine.CharacterMovementComponent|SetMaxWalkSpeed (Variables|Character|GetCharacterMovement) 4e+02)
  (if (Variables|Default|GetpawnSee)
    (AI|AIMoveTo self "0, 0, 0" (Game|GetPlayerCharacter 0) 3e+01 false)))

(event EventBeginPlay
  ;[1 1 1] Zombie가 생성될 때 Max HP로 Set
  (Variables|Default|SetCurHp (Variables|Default|GetMaxHp)))

(event Collision|EventActorBeginOverlap
  (params (OtherActor :type Actor%20Object%20Reference)))

(event EventTick
  (params (DeltaSeconds :type Float%20%28single-precision%29)))

(event EventOnDie
  ;[1 1 1] Zombie가 죽었을 때 나타나는 Effect
  (Physics|SetSimulatePhysics (Variables|Character|GetMesh) true)
  (CallFunction|DestroyCollision))

(fn ConstructionScript)